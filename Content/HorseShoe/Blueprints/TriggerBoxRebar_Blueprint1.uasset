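; Trigger volume Blueprint for the rebar stake in a horseshoe game that scores horseshoe throws landing close to it.
; On actor overlap it casts to BP_PickupHorseShoe, prints the horizontal (XY) distance between the two actor locations, and increments its Score when that is within HorseShoeRadius.
; The distance is checked only at the moment overlap begins, not where the horseshoe comes to rest.
; An explosion sound node is present but unconnected.
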(event `self.ReceiveActorBeginOverlap`
  (params (OtherActor :type "Actor Object Reference"))
  ;[1 1 1] Add to Score on Collision
  (bind _asbp_pickup_horse_shoe (cast `/Game/HorseShoe/Blueprints/BP_PickupHorseShoe` OtherActor))
  (bind _returnvalue (`KismetMathLibrary.VSize2D` (- (`KismetMathLibrary.MakeVector2D` (.x (`self.K2_GetActorLocation` _asbp_pickup_horse_shoe)) (.y (`self.K2_GetActorLocation` _asbp_pickup_horse_shoe))) (`KismetMathLibrary.MakeVector2D` (.x (`self.K2_GetActorLocation` self)) (.y (`self.K2_GetActorLocation` self))))))
  (`KismetSystemLibrary.PrintString` (`KismetStringLibrary.Conv_DoubleToString` _returnvalue))
  (if (<= _returnvalue (`self.HorseShoeRadius`))
    (`/Engine/EditorBlueprintResources/StandardMacros.IncrementInt` (`self.Score`))))

(fn `UserConstructionScript`)